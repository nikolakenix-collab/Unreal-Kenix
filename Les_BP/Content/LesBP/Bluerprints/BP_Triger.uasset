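; BP_Triger is a test trigger actor whose box overlap switches a point light's color and an enum state.
; BeginPlay sets and prints three enum values in turn.
; Overlap begin and end share a boolean branch: entering turns the light green, exiting turns it blue, and each shows the enum on T1.
; Entering adds Cont1 to Cont2, while exiting increments Cont1 and prints both counters.
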(event `self.ReceiveBeginPlay`
  (bind _output_get (set `self.NewVar` "NewEnumerator0"))
  (`KismetSystemLibrary.PrintString` (`|GetEnumeratorNameAsString` _output_get))
  (bind _output_get_2 (set `self.NewVar` "NewEnumerator1"))
  (`KismetSystemLibrary.PrintString` (`|GetEnumeratorNameAsString` _output_get_2))
  (bind _output_get_3 (set `self.NewVar` "NewEnumerator2"))
  (`KismetSystemLibrary.PrintString` (`|GetEnumeratorNameAsString` _output_get_3)))

(event `self.Box.OnComponentBeginOverlap`
  (params (OverlappedComponent :type "PrimitiveComponent Object Reference") (OtherActor :type "Actor Object Reference") (OtherComp :type "PrimitiveComponent Object Reference") (OtherBodyIndex :type Integer) (bFromSweep :type Boolean) (SweepResult :type "HitResult Structure (by ref)"))
  (bind _cont1 (`self.cont1`))
  (bind _pointlight (`self.PointLight`))
  (set `self.bool_Chek1` true)
  (if (`self.bool_Chek1`) :!label _label
    (`LightComponent.SetLightColor` _pointlight (struct :`G` 1.0 :`B` 0.004494 :`A` 1.0) true)
    (bind _output_get (set `self.NewVar` "NewEnumerator1"))
    (bind _output_get_2 (set `self.cont2` (+ (`self.cont2`) _cont1)))
    (`TextRenderComponent.K2_SetText` (`self.T1`) (`|FormatText` (`KismetTextLibrary.Conv_StringToText` (`|GetEnumeratorNameAsString` _output_get))))
    (else
      (`LightComponent.SetLightColor` _pointlight (struct :`G` 0.037221 :`B` 1.0 :`A` 1.0) true)
      (bind _output_get_3 (set `self.NewVar` "NewEnumerator0"))
      (bind _result (`/Engine/EditorBlueprintResources/StandardMacros.IncrementInt` _cont1)
        (:`  `
          (for _array_element (`|MakeArray` _output_get_2 _result)
            (`KismetSystemLibrary.PrintString` "Exit:")
            (`KismetSystemLibrary.PrintString` (`KismetStringLibrary.Conv_IntToString` _array_element))
            (`TextRenderComponent.K2_SetText` (`self.T1`) (`|FormatText` (`KismetTextLibrary.Conv_StringToText` (`|GetEnumeratorNameAsString` _output_get_3))))))))))

(event `self.Box.OnComponentEndOverlap`
  (params (OverlappedComponent :type "PrimitiveComponent Object Reference") (OtherActor :type "Actor Object Reference") (OtherComp :type "PrimitiveComponent Object Reference") (OtherBodyIndex :type Integer))
  (set `self.bool_Chek1` false)
  (goto _label))

(fn `UserConstructionScript`)